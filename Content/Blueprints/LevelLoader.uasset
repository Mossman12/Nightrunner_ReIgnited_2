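; LevelLoader is a one-shot trigger that streams levels in and out when the third-person character overlaps it.
; It can teleport the player to OffsetToAdd, either directly or shifted by their horizontal entry offset within the box.
; A distance check snaps the player back to that point if they land too far away, and prints debug distances.
; It then updates the game mode's battery total from BlueBatteryUnlock actors and destroys itself.
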(event OnComponentBeginOverlap(BoxTrigger)
  (params (OverlappedComponent :type Primitive%20Component%20Object%20Reference) (OtherActor :type Actor%20Object%20Reference) (OtherComp :type Primitive%20Component%20Object%20Reference) (OtherBodyIndex :type Integer) (bFromSweep :type Boolean) (SweepResult :type Hit%20Result%20Structure%20%28by%20ref%29))
  (bind _leveltoload (Variables|Default|GetLevelToLoad))
  (bind _as_bp_third_person_character (Variables|Default|GetAs%20BP%20Third%20Person%20Character))
  (bind _offset_to_add (Variables|Default|GetOffset%20to%20add))
  (bind _boxtrigger (Variables|Default|GetBoxTrigger))
  (bind _offset_to_add_2 (Variables|Default|GetOffset%20to%20add))
  (bind _leveltounload (Variables|Default|GetLevelToUnload))
  (bind _offset_to_add_3 (Variables|Default|GetOffset%20to%20add))
  (bind _returnvalue (Transformation|GetWorldLocation _boxtrigger))
  (bind _returnvalue_2 (Transformation|GetActorLocation _as_bp_third_person_character))
  (bind _returnvalue_3 (Math|Vector|Distance(Vector) _offset_to_add_2 _returnvalue_2))
  (bind _returnvalue_4 (Math|Vector|Distance(Vector) _offset_to_add _returnvalue))
  (bind _asbp_third_person_character (Utilities|Casting|CastToBP_ThirdPersonCharacter OtherActor))
  (if (!= _leveltoload "")
    (Game|LoadStreamLevel(byName) _leveltoload true))
  (if (Variables|Default|GetAdd%20Offset)
    (if (Variables|Default|GetStraight%20Teleport%20Instead%20of%20Offset?)
      ;[1 1 1] Raw TP
      (Transformation|SetActorLocation (Variables|Default|GetAs%20BP%20Third%20Person%20Character) _offset_to_add_3 false true)
      (else
        (Utilities|FlowControl|DoOnce false
          (:Completed
            ;[1 1 1] Set actor location
            (Transformation|SetActorLocation (Variables|Default|GetAs%20BP%20Third%20Person%20Character) _offset_to_add_3 false true)
            ;[1 1 1] Add the offset so your not exactly at the spawnpoint
            (Transformation|AddActorWorldOffset (Variables|Default|GetAs%20BP%20Third%20Person%20Character) (* (- (Transformation|GetWorldLocation (Variables|Default|GetBoxTrigger)) (.Location (Collision|BreakHitResult SweepResult))) "-1.000000,-1.000000,0.000000") false true)))))
    ;[1 1 1] If teleported beyond offset, raw TP
    (if (> _returnvalue_3 _returnvalue_4)
      (Transformation|SetActorLocation (Variables|Default|GetAs%20BP%20Third%20Person%20Character) (Variables|Default|GetOffset%20to%20add) false true))
    (Development|PrintText (Utilities|Text|FormatText "Dist b/w TP and Player: {1} 
Dist b/w TP and Trigger: {2} " _returnvalue_3 _returnvalue_4) true true "(R=0.100127,G=1.000000,B=0.000000,A=1.000000)" 5e+01))
  (if (!= _leveltounload "")
    (Game|UnloadStreamLevel(byName) _leveltounload false))
  (bind _outactors (Actor|GetAllActorsOfClass "/Game/BlueprintOBJ/BlueBatteryUnlock.BlueBatteryUnlock_C"))
  (Variables|/Game/ThirdPerson/Blueprints/BP_ThirdPersonGameMode.BP_ThirdPersonGameMode_C|SetBatteries%20Total (Variables|Default|GetAs%20BP%20Third%20Person%20Game%20Mode) (Utilities|Array|Length _outactors))
  (Actor|DestroyActor))

(event EventBeginPlay
  (bind _asbp_third_person_character (Utilities|Casting|CastToBP_ThirdPersonCharacter (Game|GetPlayerCharacter 0)))
  (Variables|Default|SetAs%20BP%20Third%20Person%20Character _asbp_third_person_character)
  (bind _asbp_third_person_game_mode (Utilities|Casting|CastToBP_ThirdPersonGameMode (Game|GetGameMode)))
  (Variables|Default|SetAs%20BP%20Third%20Person%20Game%20Mode _asbp_third_person_game_mode))

(fn ConstructionScript)