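; Trigger button that operates doors whose DoorValue matches its ButtonValue when the third-person character overlaps its Box.
; A DoOnce, reset when the character leaves, limits it to one activation per entry; the Interact event is empty.
; It searches all actors of both door classes, toggling matching DoorBP doors.
; Matching DoorBP_Scaled doors only open, except value 7, which closes again after a timed delay.
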(event OnComponentBeginOverlap(Box)
  (params (OverlappedComponent :type Primitive%20Component%20Object%20Reference) (OtherActor :type Actor%20Object%20Reference) (OtherComp :type Primitive%20Component%20Object%20Reference) (OtherBodyIndex :type Integer) (bFromSweep :type Boolean) (SweepResult :type Hit%20Result%20Structure%20%28by%20ref%29))
  (Utilities|Casting|CastToBP_ThirdPersonCharacter OtherActor)
  (Utilities|FlowControl|DoOnce false
    (:Completed
      (Utilities|FlowControl|Sequence
        (:then_0
          (bind _outactors (Actor|GetAllActorsOfClass "/Game/BlueprintOBJ/DoorBP.DoorBP_C"))
          (bind _array_element (Utilities|Array|ForEachLoopwithBreak _outactors)
            (:LoopBody
              (if (== (Variables|/Game/BlueprintOBJ/DoorBP.DoorBP_C|GetDoorValue _array_element) (Variables|Default|GetButtonValue))
                (if (Variables|/Game/BlueprintOBJ/DoorBP.DoorBP_C|GetDoor%20Opened _array_element)
                  (Default|CloseDOor _array_element)
                  (Variables|/Game/BlueprintOBJ/DoorBP.DoorBP_C|SetDoor%20Opened _array_element false)
                  (else
                    (Default|OpenDoor _array_element)
                    (Variables|/Game/BlueprintOBJ/DoorBP.DoorBP_C|SetDoor%20Opened _array_element true)))))))
        (:then_1
          (bind _outactors_2 (Actor|GetAllActorsOfClass "/Game/BlueprintOBJ/DoorBP_Scaled.DoorBP_Scaled_C"))
          (bind _array_element_2 (Utilities|Array|ForEachLoopwithBreak _outactors_2)
            (:LoopBody
              (if (== (Variables|/Game/BlueprintOBJ/DoorBP_Scaled.DoorBP_Scaled_C|GetDoorValue _array_element_2) (Variables|Default|GetButtonValue))
                (if (not (Variables|/Game/BlueprintOBJ/DoorBP_Scaled.DoorBP_Scaled_C|GetDoor%20Opened _array_element_2))
                  (Default|OpenDoor _array_element_2)
                  (Variables|/Game/BlueprintOBJ/DoorBP_Scaled.DoorBP_Scaled_C|SetDoor%20Opened _array_element_2 true)
                  (if (== (Variables|/Game/BlueprintOBJ/DoorBP_Scaled.DoorBP_Scaled_C|GetDoorValue _array_element_2) 7)
                    (Utilities|FlowControl|Delay 1e+01)
                    (Default|CloseDOor _array_element_2)
                    (Variables|/Game/BlueprintOBJ/DoorBP_Scaled.DoorBP_Scaled_C|SetDoor%20Opened _array_element_2 false)))))))))))

(event OnComponentEndOverlap(Box)
  (params (OverlappedComponent :type Primitive%20Component%20Object%20Reference) (OtherActor :type Actor%20Object%20Reference) (OtherComp :type Primitive%20Component%20Object%20Reference) (OtherBodyIndex :type Integer))
  (Utilities|Casting|CastToBP_ThirdPersonCharacter OtherActor)
  (Utilities|FlowControl|DoOnce false) ; enters at Reset
)

(event EventInteract
  (params (Player :type Character%20Object%20Reference)))

(fn ConstructionScript)