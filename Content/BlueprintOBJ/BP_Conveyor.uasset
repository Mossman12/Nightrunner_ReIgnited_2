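; BP_Conveyor is a conveyor belt actor that pushes the third-person player character along the belt's forward direction at a set Speed.
; On BeginPlay it passes a scaled, negated Speed to the belt material's "Speed" parameter.
; Box overlaps flag when the player is on the belt.
; While flagged, Tick either adds a movement force divided by delta seconds or launches the character with velocity override, depending on ShouldAddForce.
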(event OnComponentBeginOverlap(Box)
  (params (OverlappedComponent :type Primitive%20Component%20Object%20Reference) (OtherActor :type Actor%20Object%20Reference) (OtherComp :type Primitive%20Component%20Object%20Reference) (OtherBodyIndex :type Integer) (bFromSweep :type Boolean) (SweepResult :type Hit%20Result%20Structure%20%28by%20ref%29))
  (Utilities|Casting|CastToBP_ThirdPersonCharacter OtherActor)
  (Variables|Default|SetplayerOnConveyor true))

(event OnComponentEndOverlap(Box)
  (params (OverlappedComponent :type Primitive%20Component%20Object%20Reference) (OtherActor :type Actor%20Object%20Reference) (OtherComp :type Primitive%20Component%20Object%20Reference) (OtherBodyIndex :type Integer))
  (Utilities|Casting|CastToBP_ThirdPersonCharacter OtherActor)
  (Variables|Default|SetplayerOnConveyor false))

(event EventBeginPlay
  (Rendering|Material|SetVectorParameterValueonMaterials (Variables|Default|GetConveyor) "Speed" (Math|Vector|MakeVector (* (Variables|Default|Getspeed) -0.0001) 0.0 0.0)))

(event EventTick
  (params (DeltaSeconds :type Float%20%28single-precision%29))
  (bind _conveyor (Variables|Default|GetConveyor))
  (bind _speed (Variables|Default|Getspeed))
  (bind _returnvalue (Math|Vector|GetForwardVector _conveyor))
  (bind _returnvalue_2 (Math|Vector|Normalize _returnvalue))
  (bind _returnvalue_3 (* _speed _returnvalue_2))
  (if (Variables|Default|GetplayerOnConveyor)
    (bind _asbp_third_person_character (Utilities|Casting|CastToBP_ThirdPersonCharacter (Game|Player|GetPlayerPawn 0)))
    (if (Variables|Default|GetShould%20Add%20Force)
      (Physics|AddForce (Variables|/Script/Engine.Character|GetCharacterMovement _asbp_third_person_character) (/ _returnvalue_3 (Utilities|Time|GetWorldDeltaSeconds)))
      (else
        ;[1 1 1] Launch
        (Character|LaunchCharacter _asbp_third_person_character _returnvalue_3 true true)))))

(fn ConstructionScript)