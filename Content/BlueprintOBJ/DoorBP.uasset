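; DoorBP is a door actor that slides a Cube component 600 units down to open and back up to close.
; OpenDoor and CloseDOor play the DoorOpenT timeline forward or in reverse to lerp the cube's relative location, each playing an air-hiss sound at a different pitch.
; When Autoclose is set, the timeline's update starts a 10-second delay that then calls CloseDOor.
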(event Custom|Close%20DOor
  (Audio|PlaySoundatLocation "/Game/Audio/air-hiss-102406_Cue.air-hiss-102406_Cue" (Transformation|GetActorLocation) "0, 0, 0" 1.0 1.5 0.0 "/Game/Audio/VampireAttenuation.VampireAttenuation" 0 0 0)
  (bind _open_track (Timeline|Door%20Open%20T Reverse)
    (:Update
      (Transformation|SetRelativeLocation (Variables|Default|GetCube) (Math|Vector|Lerp(Vector) "0, 0, 0" "0.000000,0.000000,-600.000000" _open_track) false false)
      (if (Variables|Default|GetAutoclose)
        (Utilities|FlowControl|Delay 1e+01)
        (CallFunction|CloseDOor)))))

(event Custom|Open%20Door
  (Audio|PlaySoundatLocation "/Game/Audio/air-hiss-102406_Cue.air-hiss-102406_Cue" (Transformation|GetActorLocation) "0, 0, 0" 1.0 2.5 0.0 "/Game/Audio/VampireAttenuation.VampireAttenuation" 0 0 0)
  (bind _open_track (Timeline|Door%20Open%20T Play)
    (:Update
      (Transformation|SetRelativeLocation (Variables|Default|GetCube) (Math|Vector|Lerp(Vector) "0, 0, 0" "0.000000,0.000000,-600.000000" _open_track) false false)
      (if (Variables|Default|GetAutoclose)
        (Utilities|FlowControl|Delay 1e+01)
        (CallFunction|CloseDOor)))))

(fn ConstructionScript)