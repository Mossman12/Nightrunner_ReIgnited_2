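; BP_MovingRock is a rock actor that moves along the world Z axis relative to where it starts.
; On BeginPlay it stores its location, waits OffsetTime, then plays a Timeline at a rate set by SpeedMulti.
; Each update scales the track value by DistanceToMove and adds it to the stored location, without sweep, so offset, speed and travel distance are driven by variables.
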(event EventBeginPlay
  (Variables|Default|SetOriginalLocation (Transformation|GetActorLocation))
  (Utilities|FlowControl|Delay (Variables|Default|GetOffsetTime))
  (Components|Timeline|SetPlayRate (Variables|Default|GetTimeline) (Variables|Default|GetSpeedMulti))
  (bind _newtrack_0 (Timeline|Timeline Play)
    (:Update
      (Transformation|SetActorLocation (+ (Math|Vector|MakeVector 0.0 0.0 (* _newtrack_0 (Variables|Default|GetDistanceToMove))) (Variables|Default|GetOriginalLocation)) false false))))

(fn ConstructionScript)