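; Grapple constraint actor that anchors a hook point and a player point for the third-person character's grapple, alongside a physics constraint.
; BeginPlay moves the constraint to the character's mesh and attaches the player point to the right-hand socket.
; While a hook exists, BeginPlay and Tick move the hook point to the grapple location.
; A one-time sphere trace there attaches the hook point to any component it hits.
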(event EventBeginPlay
  (bind _hookpoint (Variables|Default|GetHookPoint))
  (bind _returnvalue (Transformation|GetWorldLocation _hookpoint))
  (bind _asbp_third_person_character (Utilities|Casting|CastToBP_ThirdPersonCharacter (Game|GetPlayerCharacter 0)))
  (Variables|Default|SetThirdPersonChara _asbp_third_person_character)
  (Transformation|SetWorldLocation (Variables|Default|GetPhysicsConstraint) (Transformation|GetWorldLocation (Variables|/Script/Engine.Character|GetMesh (Variables|Default|GetThirdPersonChara))) false true)
  (Transformation|SetWorldLocation (Variables|Default|GetPlayerPoint) (Transformation|GetWorldLocation (Variables|/Script/Engine.Character|GetMesh (Variables|Default|GetThirdPersonChara))) false true)
  (Transformation|AttachComponentToComponent (Variables|Default|GetPlayerPoint) (Variables|/Script/Engine.Character|GetMesh (Variables|Default|GetThirdPersonChara)) "hand_r" "SnapToTarget" "SnapToTarget" "SnapToTarget" true)
  ;[1 1 1] Attach Hook
  (if (Variables|/Game/ThirdPerson/Blueprints/BP_ThirdPersonCharacter.BP_ThirdPersonCharacter_C|GetCreated%20Hook (Variables|Default|GetThirdPersonChara))
    (bind _returnvalue_2 (Actor|GetActorOfClass "/Game/BlueprintOBJ/HookHeadObj.HookHeadObj_C"))
    (Variables|Default|SetHookHeadObj _returnvalue_2)
    (Transformation|SetWorldLocation _hookpoint (Variables|/Game/ThirdPerson/Blueprints/BP_ThirdPersonCharacter.BP_ThirdPersonCharacter_C|GetGrapplePoint (Variables|Default|GetThirdPersonChara)) false false)
    (Utilities|FlowControl|DoOnce false
      (:Completed
        (bind (_outhit _returnvalue_3) (Collision|SphereTraceByChannel _returnvalue _returnvalue 2e+01 "TraceTypeQuery1" false 0 "ForDuration"))
        (if _returnvalue_3
          (Development|PrintString "Hello From Constraint")
          (Transformation|AttachComponentToComponent (Variables|Default|GetHookPoint) (.HitComponent (Collision|BreakHitResult _outhit)) "None" "KeepWorld" "KeepRelative" "KeepWorld" true))))))

(event Collision|EventActorBeginOverlap
  (params (OtherActor :type Actor%20Object%20Reference)))

(event EventTick
  (params (DeltaSeconds :type Float%20%28single-precision%29))
  (bind _hookpoint (Variables|Default|GetHookPoint))
  (bind _returnvalue (Transformation|GetWorldLocation _hookpoint))
  ;[1 1 1] Attach Hook
  (if (Variables|/Game/ThirdPerson/Blueprints/BP_ThirdPersonCharacter.BP_ThirdPersonCharacter_C|GetCreated%20Hook (Variables|Default|GetThirdPersonChara))
    (bind _returnvalue_2 (Actor|GetActorOfClass "/Game/BlueprintOBJ/HookHeadObj.HookHeadObj_C"))
    (Variables|Default|SetHookHeadObj _returnvalue_2)
    (Transformation|SetWorldLocation _hookpoint (Variables|/Game/ThirdPerson/Blueprints/BP_ThirdPersonCharacter.BP_ThirdPersonCharacter_C|GetGrapplePoint (Variables|Default|GetThirdPersonChara)) false false)
    (Utilities|FlowControl|DoOnce false
      (:Completed
        (bind (_outhit _returnvalue_3) (Collision|SphereTraceByChannel _returnvalue _returnvalue 2e+01 "TraceTypeQuery1" false 0 "ForDuration"))
        (if _returnvalue_3
          (Development|PrintString "Hello From Constraint")
          (Transformation|AttachComponentToComponent (Variables|Default|GetHookPoint) (.HitComponent (Collision|BreakHitResult _outhit)) "None" "KeepWorld" "KeepRelative" "KeepWorld" true))))))

(fn ConstructionScript)