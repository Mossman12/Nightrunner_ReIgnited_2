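; BP_HoverBoard is a rideable board that the third-person character moves by standing on its left or right side.
; Overlaps on LeftBox and RightBox set direction flags, and Tick moves the board along the mesh's forward axis while tilting the Scene component.
; When the player gets farther than RespawnDistance, the board teleports back to its starting location.
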(event OnComponentBeginOverlap(LeftBox)
  (params (OverlappedComponent :type Primitive%20Component%20Object%20Reference) (OtherActor :type Actor%20Object%20Reference) (OtherComp :type Primitive%20Component%20Object%20Reference) (OtherBodyIndex :type Integer) (bFromSweep :type Boolean) (SweepResult :type Hit%20Result%20Structure%20%28by%20ref%29))
  (Utilities|Casting|CastToBP_ThirdPersonCharacter OtherActor)
  (Variables|Default|SetOnLeft true))

(event OnComponentEndOverlap(LeftBox)
  (params (OverlappedComponent :type Primitive%20Component%20Object%20Reference) (OtherActor :type Actor%20Object%20Reference) (OtherComp :type Primitive%20Component%20Object%20Reference) (OtherBodyIndex :type Integer))
  (Utilities|Casting|CastToBP_ThirdPersonCharacter OtherActor)
  (Variables|Default|SetOnLeft false))

(event OnComponentBeginOverlap(RightBox)
  (params (OverlappedComponent :type Primitive%20Component%20Object%20Reference) (OtherActor :type Actor%20Object%20Reference) (OtherComp :type Primitive%20Component%20Object%20Reference) (OtherBodyIndex :type Integer) (bFromSweep :type Boolean) (SweepResult :type Hit%20Result%20Structure%20%28by%20ref%29))
  (Utilities|Casting|CastToBP_ThirdPersonCharacter OtherActor)
  (Variables|Default|SetOnRight true))

(event OnComponentEndOverlap(RightBox)
  (params (OverlappedComponent :type Primitive%20Component%20Object%20Reference) (OtherActor :type Actor%20Object%20Reference) (OtherComp :type Primitive%20Component%20Object%20Reference) (OtherBodyIndex :type Integer))
  (Utilities|Casting|CastToBP_ThirdPersonCharacter OtherActor)
  (Variables|Default|SetOnRight false))

(event EventBeginPlay
  (Variables|Default|SetInitial (Transformation|GetActorLocation))
  (bind _asbp_third_person_character (Utilities|Casting|CastToBP_ThirdPersonCharacter (Game|Player|GetPlayerPawn 0)))
  (Variables|Default|SetAs%20BP%20Third%20Person%20Character _asbp_third_person_character))

(event EventTick
  (params (DeltaSeconds :type Float%20%28single-precision%29))
  (bind _speed (Variables|Default|GetSpeed))
  (bind _staticmesh1 (Variables|Default|GetStaticMesh1))
  (bind _returnvalue (Math|Vector|GetForwardVector _staticmesh1))
  (bind _returnvalue_2 (* DeltaSeconds _speed))
  (bind _returnvalue_3 (* _returnvalue _returnvalue_2))
  (Utilities|IsValid (Variables|Default|GetAs%20BP%20Third%20Person%20Character)
    (:Is%20Valid
      (Utilities|FlowControl|Sequence
        (:then_0
          (if (Variables|Default|GetOnLeft)
            (Transformation|SetActorLocation (- (Transformation|GetActorLocation) _returnvalue_3) false false)
            (Transformation|SetRelativeRotation (Variables|Default|GetScene) "3.000000,0.000000,0.000000" false false)
            (elif (Variables|Default|GetOnRight)
              (Transformation|SetActorLocation (+ _returnvalue_3 (Transformation|GetActorLocation)) false false)
              (Transformation|SetRelativeRotation (Variables|Default|GetScene) "-3.000000,0.000000,0.000000" false false))))
        (:then_1
          (if (and (> (Math|Vector|Distance(Vector) (Transformation|GetActorLocation (Variables|Default|GetAs%20BP%20Third%20Person%20Character)) (Transformation|GetActorLocation)) (Variables|Default|GetRespawnDistance)) (Utilities|Operators|NotEqual(!=) (Transformation|GetActorLocation) (Variables|Default|GetInitial) 1.0))
            (Transformation|SetActorLocation (Variables|Default|GetInitial) false false)))))))

(fn ConstructionScript)