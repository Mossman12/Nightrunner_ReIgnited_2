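; GrappleAquireDoorBP is a door that slides its cube down to open and back up to close.
; OpenDoor passes a do-once gate, then plays an air-hiss sound and a timeline that lerps the cube's relative location.
; CloseDOor reverses that timeline with a lower-pitched hiss, while UnlockDoor resets the gate once enough bats are counted.
; The delayed auto-close logic is disconnected and never runs.
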(event Custom|Unlock%20Door
  (if (>= (Variables|Default|GetTotalBats) 3)
    (Utilities|FlowControl|DoOnce false) ; enters at Reset
  ))

(event Custom|Close%20DOor
  (Variables|Default|SetDoor%20has%20been%20Opened%20and%20Closed? true)
  (Audio|PlaySoundatLocation "/Game/Audio/air-hiss-102406_Cue.air-hiss-102406_Cue" (Transformation|GetActorLocation) "0, 0, 0" 1.0 1.5 0.0 "/Game/Audio/VampireAttenuation.VampireAttenuation" 0 0 0)
  (bind _open_track (Timeline|Door%20Open%20T Reverse)
    (:Update
      (Transformation|SetRelativeLocation (Variables|Default|GetCube) (Math|Vector|Lerp(Vector) "0, 0, 0" "0.000000,0.000000,-600.000000" _open_track) false false)
      (if (Variables|Default|GetDoor%20has%20been%20Opened%20and%20Closed?)
        _))))

(event Custom|Open%20Door
  (Utilities|FlowControl|DoOnce false
    (:Completed
      (Audio|PlaySoundatLocation "/Game/Audio/air-hiss-102406_Cue.air-hiss-102406_Cue" (Transformation|GetActorLocation) "0, 0, 0" 1.0 2.5 0.0 "/Game/Audio/VampireAttenuation.VampireAttenuation" 0 0 0)
      (bind _open_track (Timeline|Door%20Open%20T Play)
        (:Update
          (Transformation|SetRelativeLocation (Variables|Default|GetCube) (Math|Vector|Lerp(Vector) "0, 0, 0" "0.000000,0.000000,-600.000000" _open_track) false false)
          (if (Variables|Default|GetDoor%20has%20been%20Opened%20and%20Closed?)
            _))))))

(fn ConstructionScript)