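; Battery-powered lock button that opens its matching door once the player has collected the required number of batteries.
; On Interact it compares the game mode's battery count to BatteryNeeded, showing a subtitle hint when they differ.
; On success, chained timelines swap the empty battery and rotate the glass, then delayed material changes light the gauges.
; It then plays a sound and opens the DoorBP whose DoorValue matches ButtonValue.
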(event EventInteract
  (params (Player :type Character%20Object%20Reference))
  (bind _material (Variables|Default|GetMaterial))
  (bind _batteryneeded (Variables|Default|GetBatteryNeeded))
  (bind _asbp_third_person_game_mode (Utilities|Casting|CastToBP_ThirdPersonGameMode (Game|GetGameMode)))
  (Variables|/Game/ThirdPerson/Blueprints/BP_ThirdPersonGameMode.BP_ThirdPersonGameMode_C|SetBatteries%20Left _asbp_third_person_game_mode _batteryneeded)
  (if (== (Variables|/Game/ThirdPerson/Blueprints/BP_ThirdPersonGameMode.BP_ThirdPersonGameMode_C|GetBatteries%20Collected _asbp_third_person_game_mode) _batteryneeded)
    (bind _take_out_battery (Timeline|Move%20Empty%20Battery Play)
      (:Update
        (Transformation|SetRelativeLocation (Variables|Default|GetEmptyBattery) (Math|Vector|Lerp(Vector) "0.000000,-35.000000,10.000000" "0.000000,100.000000,0.000000" _take_out_battery) false false))
      (:Finished
        (Transformation|SetRelativeLocationAndRotation (Variables|Default|GetEmptyBattery) (Variables|Default|GetEmpty%20Rest%20Location) (Variables|Default|GetEmpty%20Rest%20Rotation) false false)
        (Utilities|FlowControl|Delay 0.75)
        (Rendering|SetVisibility (Variables|Default|GetExample_Battery) true false)
        (bind _take_out_battery_2 (Timeline|Insert%20Battery Play)
          (:Update
            (Transformation|SetRelativeLocation (Variables|Default|GetExample_Battery) (Math|Vector|Lerp(Vector) "0.000000,-35.000000,10.000000" "0.000000,100.000000,0.000000" _take_out_battery_2) false false))
          (:Finished
            (Utilities|FlowControl|Delay 0.5)
            (bind _rotate_glass (Timeline|Rotate%20Glass Play)
              (:Update
                (Transformation|SetRelativeRotation (Variables|Default|GetGlass) (Math|Rotator|Lerp(Rotator) "0.000000,0.000000,-160.000000" "0.000000,0.000000,90.000000" _rotate_glass) false false))
              (:Finished
                ;[1 1 1] Change Mats for Meter
                (Utilities|FlowControl|Delay 0.3)
                (Rendering|Material|SetMaterial (Variables|Default|GetPower%20Gauge%201) 0 _material)
                (Utilities|FlowControl|Delay 0.1)
                (Rendering|Material|SetMaterial (Variables|Default|GetPower%20Gauge%202) 0 _material)
                (Rendering|Material|SetMaterial (Variables|Default|GetPipe) 0 "/Game/BlueprintOBJ/StuffIAdded/TransparentBackCulling_3.TransparentBackCulling_3")
                (Utilities|FlowControl|Delay 0.1)
                (Rendering|Material|SetMaterial (Variables|Default|GetPower%20Gauge%203) 0 _material)
                (Rendering|Material|SetMaterial (Variables|Default|GetPipe) 0 "/Game/BlueprintOBJ/StuffIAdded/TransparentBackCulling_7.TransparentBackCulling_7")
                (Utilities|FlowControl|Delay 0.1)
                (Rendering|Material|SetMaterial (Variables|Default|GetPower%20Gauge%204) 0 _material)
                (Rendering|Material|SetMaterial (Variables|Default|GetPipe) 0 _material)
                ;[1 1 1] Set Materials
                (Utilities|FlowControl|Delay 0.1)
                (Rendering|Material|SetMaterial (Variables|Default|GetBacking%20Plane) 0 "/Game/StarterContent/Materials/M_Tech_Hex_Tile_Pulse.M_Tech_Hex_Tile_Pulse")
                (Rendering|Material|SetMaterial (Variables|Default|GetBacking%20Plane1) 0 "/Game/StarterContent/Materials/M_Tech_Hex_Tile_Pulse.M_Tech_Hex_Tile_Pulse")
                (Rendering|Material|SetMaterial (Variables|Default|GetBacking%20Plane2) 0 "/Game/StarterContent/Materials/M_Tech_Hex_Tile_Pulse.M_Tech_Hex_Tile_Pulse")
                (Rendering|Material|SetMaterial (Variables|Default|GetBacking%20Plane3) 0 "/Game/StarterContent/Materials/M_Tech_Hex_Tile_Pulse.M_Tech_Hex_Tile_Pulse")
                ;[1 1 1] CONGRUNTILARION
                (Utilities|FlowControl|Delay 0.2)
                (Audio|PlaySound2D "/Game/Audio/CONGRUNTILARION.CONGRUNTILARION" 1.0 1.0 0.0 0 0)
                (Utilities|FlowControl|Delay 0.2)
                ;[1 1 1] Open Door
                (bind _outactors (Actor|GetAllActorsOfClass "/Game/BlueprintOBJ/DoorBP.DoorBP_C"))
                (bind _array_element (Utilities|Array|ForEachLoopwithBreak _outactors :!label _label)
                  (:LoopBody
                    (if (== (Variables|/Game/BlueprintOBJ/DoorBP.DoorBP_C|GetDoorValue _array_element) (Variables|Default|GetButtonValue))
                      (Default|OpenDoor _array_element)
                      (bind _returnvalue (UserInterface|CreateWidget "/Game/ThirdPerson/Blueprints/Subtitle_UI_Widget.Subtitle_UI_Widget_C"))
                      (Default|SayText _returnvalue (Utilities|Text|FormatText "This isn't my finest work, but if it works. ") 7.0 false)
                      (UserInterface|Viewport|AddtoViewport _returnvalue 0)
                      (goto _label Break))))))))))
    (elif (== (Variables|/Game/ThirdPerson/Blueprints/BP_ThirdPersonGameMode.BP_ThirdPersonGameMode_C|GetBatteries%20Collected _asbp_third_person_game_mode) 1)
      ;[1 1 1] If you have NO batteries
      (bind _returnvalue_2 (UserInterface|CreateWidget "/Game/ThirdPerson/Blueprints/Subtitle_UI_Widget.Subtitle_UI_Widget_C"))
      (Default|SayText _returnvalue_2 (Utilities|Text|FormatText "Gonna need to hope theres enough batteries 
out in The Junkfield to jumpstart this.  
I'm gonna need {X} more..." (- _batteryneeded (Variables|/Game/ThirdPerson/Blueprints/BP_ThirdPersonGameMode.BP_ThirdPersonGameMode_C|GetBatteries%20Collected _asbp_third_person_game_mode))) 7.0 false)
      (UserInterface|Viewport|AddtoViewport _returnvalue_2 0)
      (else
        ;[1 1 1] If you have 1 battery
        (bind _returnvalue_3 (UserInterface|CreateWidget "/Game/ThirdPerson/Blueprints/Subtitle_UI_Widget.Subtitle_UI_Widget_C"))
        (Default|SayText _returnvalue_3 (Utilities|Text|FormatText "I'm gonna need more batteries...") 7.0 false)
        (UserInterface|Viewport|AddtoViewport _returnvalue_3 0)))))

(fn ConstructionScript)