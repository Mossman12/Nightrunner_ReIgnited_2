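; ButtonCloseOnlyCollideBP is a collision-triggered button that only closes doors.
; When BP_ThirdPersonCharacter overlaps its Box, it searches every DoorBP for a DoorValue matching its ButtonValue.
; An open match is closed and marked closed through a DoOnce, which resets when a matching door is found already closed.
; Interact and end overlap are empty, and the button animation, material and door-opening nodes are disconnected.
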(event OnComponentBeginOverlap(Box)
  (params (OverlappedComponent :type Primitive%20Component%20Object%20Reference) (OtherActor :type Actor%20Object%20Reference) (OtherComp :type Primitive%20Component%20Object%20Reference) (OtherBodyIndex :type Integer) (bFromSweep :type Boolean) (SweepResult :type Hit%20Result%20Structure%20%28by%20ref%29))
  (Utilities|Casting|CastToBP_ThirdPersonCharacter OtherActor)
  (bind _outactors (Actor|GetAllActorsOfClass "/Game/BlueprintOBJ/DoorBP.DoorBP_C"))
  (bind _array_element (Utilities|Array|ForEachLoopwithBreak _outactors)
    (:LoopBody
      (if (== (Variables|/Game/BlueprintOBJ/DoorBP.DoorBP_C|GetDoorValue _array_element) (Variables|Default|GetButtonValue))
        (if (Variables|/Game/BlueprintOBJ/DoorBP.DoorBP_C|GetDoor%20Opened _array_element)
          (Utilities|FlowControl|DoOnce false :!label _label
            (:Completed
              (Default|CloseDOor _array_element)
              (Variables|/Game/BlueprintOBJ/DoorBP.DoorBP_C|SetDoor%20Opened _array_element false)))
          (else
            (goto _label Reset)))))))

(event OnComponentEndOverlap(Box)
  (params (OverlappedComponent :type Primitive%20Component%20Object%20Reference) (OtherActor :type Actor%20Object%20Reference) (OtherComp :type Primitive%20Component%20Object%20Reference) (OtherBodyIndex :type Integer)))

(event EventInteract
  (params (Player :type Character%20Object%20Reference)))

(fn ConstructionScript)