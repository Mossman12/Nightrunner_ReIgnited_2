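; Behavior tree task that makes a Vampire chase the player, with sound, light and music feedback.
; On execute it stops one music cue, plays a chase sound and burst, then runs AIMoveTo on the player while showing fangs, tinting the light and starting drums.
; Catching the player spawns a blood burst and calls KILLNIGEL after a delay; failure resets fangs and light.
; The task never calls Finish Execute.
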(event EventReceiveExecuteAI
  (params (OwnerController :type AI%20Controller%20Object%20Reference) (ControlledPawn :type Pawn%20Object%20Reference))
  (bind _returnvalue (Game|GetPlayerCharacter 0))
  (bind _asvampire (Utilities|Casting|CastToVampire ControlledPawn))
  (Variables|Default|SetAs%20Vampire _asvampire)
  (bind _asbp_third_person_character (Utilities|Casting|CastToBP_ThirdPersonCharacter (Game|GetPlayerCharacter 0)))
  (Variables|Default|SetAs%20BP%20Third%20Person%20Character _asbp_third_person_character)
  (Audio|Components|Audio|Stop (Variables|/Game/AI/Vampire.Vampire_C|GetPepper_Steak_End_Cue (Variables|Default|GetAs%20Vampire)))
  ;[1 1 1] Play Chase Sound
  (Audio|PlaySoundatLocation "/Game/Audio/VampireCue.VampireCue" (Transformation|GetActorLocation (Variables|Default|GetAs%20Vampire)) (Transformation|GetActorRotation (Variables|Default|GetAs%20Vampire)) 1.0 1.0 0.0 "/Game/Audio/VampireAttenuation.VampireAttenuation" 0 (Variables|Default|GetAs%20Vampire) 0)
  (Default|DETECTEDBurst (Variables|Default|GetAs%20Vampire))
  (AI|AIMoveTo (Variables|Default|GetAs%20Vampire) (Transformation|GetWorldLocation (Variables|/Script/Engine.Character|GetMesh _returnvalue)) _returnvalue 0.0 false
    (:then
      ;[1 1 1] While Chase
      (Variables|/Game/AI/Vampire.Vampire_C|SetVampire%20Chase%20Bool (Variables|Default|GetAs%20Vampire) true)
      (Rendering|SetVisibility (Variables|/Game/AI/Vampire.Vampire_C|Getfang (Variables|Default|GetAs%20Vampire)) true false)
      (Rendering|Components|Light|SetLightColor (Variables|/Game/AI/Vampire.Vampire_C|GetPointLight (Variables|Default|GetAs%20Vampire)) "(R=0.045641,G=0.000000,B=0.090196,A=1.000000)" true)
      (Rendering|Components|Light|SetIntensity (Variables|/Game/AI/Vampire.Vampire_C|GetPointLight (Variables|Default|GetAs%20Vampire)) 1e+05)
      ;[1 1 1] If Drums are not playing, play drums
      (if (not (Audio|Components|Audio|IsPlaying (Variables|/Game/AI/Vampire.Vampire_C|GetPepper_Steak_End_Drums_Cue (Variables|Default|GetAs%20Vampire))))
        (Audio|Components|Audio|Play (Variables|/Game/AI/Vampire.Vampire_C|GetPepper_Steak_End_Drums_Cue (Variables|Default|GetAs%20Vampire)) 0.0)))
    (:OnSuccess
      ;[1 1 1] On Cactch
      ;;[1 1 1] Caught Them
      (Rendering|Components|Light|SetLightColor (Variables|/Game/AI/Vampire.Vampire_C|GetPointLight (Variables|Default|GetAs%20Vampire)) "(R=4.000000,G=0.000000,B=0.131313,A=1.000000)" true)
      ;;[1 1 1] Trigger this and respawn (Done Elsewhere RN)
      (Niagara|SpawnSystemAttached "/Game/Niagara_Particles/BloodBurst.BloodBurst" (Variables|/Script/Engine.Character|GetMesh (Game|GetPlayerCharacter 0)) "None" "0.000000,0.000000,10.000000" "0, 0, 0" "KeepRelativeOffset" true)
      (Utilities|FlowControl|Delay 1.0)
      (Default|KILLNIGEL (Variables|Default|GetAs%20Vampire)))
    (:OnFail
      ;[1 1 1] Lost Em
      (Rendering|Components|Light|SetLightColor (Variables|/Game/AI/Vampire.Vampire_C|GetPointLight (Variables|Default|GetAs%20Vampire)) "(R=0.000000,G=0.000000,B=0.000000,A=0.149000)" true)
      (Rendering|SetVisibility (Variables|/Game/AI/Vampire.Vampire_C|Getfang (Variables|Default|GetAs%20Vampire)) false false))))